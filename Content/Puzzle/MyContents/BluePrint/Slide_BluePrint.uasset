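; Sliding trigger actor for a puzzle level that pushes the player pawn along while an overlap is active.
; Begin overlap sets an IsOver flag and prints a debug message; end overlap and BeginPlay clear it.
; While the flag is set, Tick moves player 0's pawn a fixed step along its local X axis with sweep and teleport, unscaled by delta time.
; The overlapping actor is never checked.
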(event `self.ReceiveTick`
  (params (DeltaSeconds :type "Float (single-precision)"))
  (if (`self.isOver`)
    (bind _output_get (set `self.nextBlock` (+ (0.0 0.0 0.0) (8.0 0.0 0.0))))
    (`self.K2_AddActorLocalOffset` (`GameplayStatics.GetPlayerPawn` 0) _output_get true true) ; 움직이는 방향으로 이동
    (else
      (set `self.nextBlock` (`self.K2_GetActorLocation`)))))

(event `self.ReceiveBeginPlay`
  (set `self.isOver` false :!label _label))

(event `self.ReceiveActorEndOverlap`
  (params (OtherActor :type "Actor Object Reference"))
  (goto _label))

(event `self.ReceiveActorBeginOverlap`
  (params (OtherActor :type "Actor Object Reference"))
  (if (not (`self.isOver`))
    (`KismetSystemLibrary.PrintString` "Sliding")
    (set `self.isOver` true)))

(fn `UserConstructionScript`)