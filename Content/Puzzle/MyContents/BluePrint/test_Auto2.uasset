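; A test puzzle interaction actor that swaps its Image component for a Complete component once its activation conditions are met.
; A Sphere overlap toggles the prompt Text and the IsNear flag, without filtering the overlapping actor.
; Tick polls IsNear, IsHand and IsPressed, then prints, hides Image and shows Complete with physics-only collision.
; IsHand and IsPressed are only reset at BeginPlay, never set true here.
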(event `self.ReceiveBeginPlay`
  (bind _complete (`self.Complete`))
  (set `self.isHand` false)
  (set `self.isNear` false)
  (set `self.isPressed` false)
  (`SceneComponent.SetVisibility` _complete false false)
  (`PrimitiveComponent.SetCollisionEnabled` _complete "NoCollision"))

(event `self.ReceiveActorBeginOverlap`
  (params (OtherActor :type "Actor Object Reference")))

(event `self.Sphere.OnComponentBeginOverlap`
  (params (OverlappedComponent :type "PrimitiveComponent Object Reference") (OtherActor :type "Actor Object Reference") (OtherComp :type "PrimitiveComponent Object Reference") (OtherBodyIndex :type Integer) (bFromSweep :type Boolean) (SweepResult :type "HitResult Structure (by ref)"))
  (`SceneComponent.SetVisibility` (`self.Text`) true false)
  (set `self.isNear` true))

(event `self.Sphere.OnComponentEndOverlap`
  (params (OverlappedComponent :type "PrimitiveComponent Object Reference") (OtherActor :type "Actor Object Reference") (OtherComp :type "PrimitiveComponent Object Reference") (OtherBodyIndex :type Integer))
  (`SceneComponent.SetVisibility` (`self.Text`) false false)
  (set `self.isNear` false))

(event `self.ReceiveTick`
  (params (DeltaSeconds :type "Float (single-precision)"))
  (bind _complete (`self.Complete`))
  (if (`self.isNear`)
    (if (`self.isHand`)
      (if (`self.isPressed`)
        (`KismetSystemLibrary.PrintString` "press")
        (`SceneComponent.SetVisibility` _complete true false)
        (`SceneComponent.SetVisibility` (`self.Image`) false false)
        (`PrimitiveComponent.SetCollisionEnabled` _complete "PhysicsOnly")))))

(fn `UserConstructionScript`)