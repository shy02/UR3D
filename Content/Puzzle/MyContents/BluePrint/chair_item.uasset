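; Chair item pickup actor for a puzzle game that can be collected when the player is nearby.
; A sphere overlap shows or hides a text component and tracks proximity in IsNear.
; Tick polls IsPressedI, which nothing here sets to true, together with IsNear.
; When both are true, it sets IsHand on the Chair actor found by class, plays a 2D sound and destroys itself.
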(event `self.ReceiveActorBeginOverlap`
  (params (OtherActor :type "Actor Object Reference")))

(event `self.ReceiveBeginPlay`
  (set `self.isPressed_i` false)
  (set `self.isNear` false))

(event `self.ReceiveTick`
  (params (DeltaSeconds :type "Float (single-precision)"))
  (if (`self.isPressed_i`)
    (if (`self.isNear`)
      (bind _returnvalue (`GameplayStatics.GetActorOfClass` "/Game/Puzzle/MyContents/BluePrint/chair.chair_C"))
      (set `/Game/Puzzle/MyContents/BluePrint/chair.isHand` true _returnvalue)
      (`GameplayStatics.PlaySound2D` "/Game/JGM/sound/thiring2.thiring2" 1.0 1.0 0.0 null null)
      (`self.K2_DestroyActor`))))

(event `self.Sphere.OnComponentBeginOverlap`
  (params (OverlappedComponent :type "PrimitiveComponent Object Reference") (OtherActor :type "Actor Object Reference") (OtherComp :type "PrimitiveComponent Object Reference") (OtherBodyIndex :type Integer) (bFromSweep :type Boolean) (SweepResult :type "HitResult Structure (by ref)"))
  (`SceneComponent.SetVisibility` (`self.Text`) true false)
  (set `self.isNear` true))

(event `self.Sphere.OnComponentEndOverlap`
  (params (OverlappedComponent :type "PrimitiveComponent Object Reference") (OtherActor :type "Actor Object Reference") (OtherComp :type "PrimitiveComponent Object Reference") (OtherBodyIndex :type Integer))
  (`SceneComponent.SetVisibility` (`self.Text`) false false)
  (set `self.isNear` false))

(fn `UserConstructionScript`)