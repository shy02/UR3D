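; Pressure-plate Blueprint that signals the puzzle wall when an actor steps on it.
; At BeginPlay it hides the Stepped mesh; on overlap it swaps the Cube for Stepped and prints "Open".
; It then finds a Wall_BluePrint with GetActorOfClass and sets its IsStepped flag.
; The IsOver guard is never set true here, so every overlap repeats this, and leaving the plate does nothing.
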(event `self.ReceiveBeginPlay`
  (set `self.isOver` false)
  (`SceneComponent.SetVisibility` (`self.stepped`) false false))

(event `self.ReceiveActorEndOverlap`
  (params (OtherActor :type "Actor Object Reference")))

(event `self.ReceiveActorBeginOverlap`
  (params (OtherActor :type "Actor Object Reference"))
  (if (not (`self.isOver`))
    (`SceneComponent.SetVisibility` (`self.Cube`) false false)
    (`SceneComponent.SetVisibility` (`self.stepped`) true false)
    (`KismetSystemLibrary.PrintString` "Open")
    (bind _returnvalue (`GameplayStatics.GetActorOfClass` "/Game/Puzzle/MyContents/BluePrint/Wall_BluePrint.Wall_BluePrint_C"))
    (bind _aswall_blue_print (cast `/Game/Puzzle/MyContents/BluePrint/Wall_BluePrint` _returnvalue))
    (set `/Game/Puzzle/MyContents/BluePrint/Wall_BluePrint.isStepped` true _aswall_blue_print)))

(fn `UserConstructionScript`)