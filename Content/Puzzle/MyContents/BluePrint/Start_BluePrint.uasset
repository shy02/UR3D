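; Start-zone actor for a puzzle course that starts the on-screen timer as something leaves it.
; The first overlap, gated by IsTimerExist and IsOver, creates the Timer widget, adds it to the viewport and pauses its Timer_ function timer.
; Ending an overlap unpauses that timer and hands the widget to every End_BluePrint actor through its Obj variable.
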(event `self.ReceiveBeginPlay`
  (set `self.isOver` false))

(event `self.ReceiveActorEndOverlap`
  (params (OtherActor :type "Actor Object Reference"))
  (`KismetSystemLibrary.K2_UnPauseTimer` (`self.timer_obj`) "Timer_")
  (bind _outactors (`GameplayStatics.GetAllActorsOfClass` "/Game/Puzzle/MyContents/BluePrint/End_BluePrint.End_BluePrint_C"))
  (for _array_element _outactors
    (bind _asend_blue_print (cast `/Game/Puzzle/MyContents/BluePrint/End_BluePrint` _array_element :!label _label))
    (set `/Game/Puzzle/MyContents/BluePrint/End_BluePrint.obj` (`self.timer_obj`) _asend_blue_print))
  (goto _label))

(event `self.ReceiveActorBeginOverlap`
  (params (OtherActor :type "Actor Object Reference"))
  (if (`self.isOver`)
    _
    (elif (not (`self.isTimerExist`))
      (`KismetSystemLibrary.PrintString` "Timer Start")
      (set `self.isTimerExist` true)
      (bind _returnvalue (`|CreateWidget` "/Game/Puzzle/MyContents/BluePrint/Timer.Timer_C"))
      (bind _output_get (set `self.timer_obj` _returnvalue))
      (`UserWidget.AddToViewport` _output_get 0)
      (`KismetSystemLibrary.K2_PauseTimer` (`self.timer_obj`) "Timer_"))))

(fn `UserConstructionScript`)