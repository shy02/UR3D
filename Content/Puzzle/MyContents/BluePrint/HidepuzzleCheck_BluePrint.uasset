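; Hide puzzle checker actor that flags the puzzle as finished and shows a text prompt when the player is nearby.
; A sphere overlap shows the Text for the grab first-person character and hides it on exit; it starts hidden.
; Tick polls the CheckB, CheckC and CheckP flags, which this graph never sets, and when all are true sets IsEnd and hides the Text.
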(event `self.ReceiveBeginPlay`
  (`SceneComponent.SetVisibility` (`self.text`) false false))

(event `self.ReceiveTick`
  (params (DeltaSeconds :type "Float (single-precision)"))
  (if (`self.check_b`)
    (if (`self.check_c`)
      (if (`self.check_p`)
        (set `self.isEnd` true)
        (`SceneComponent.SetVisibility` (`self.text`) false false)))))

(event `self.Sphere.OnComponentBeginOverlap`
  (params (OverlappedComponent :type "PrimitiveComponent Object Reference") (OtherActor :type "Actor Object Reference") (OtherComp :type "PrimitiveComponent Object Reference") (OtherBodyIndex :type Integer) (bFromSweep :type Boolean) (SweepResult :type "HitResult Structure (by ref)"))
  (cast `/Game/FirstPerson/Blueprints/BP_FirstPersonCharacter_Grab` OtherActor)
  (`SceneComponent.SetVisibility` (`self.text`) true false))

(event `self.Sphere.OnComponentEndOverlap`
  (params (OverlappedComponent :type "PrimitiveComponent Object Reference") (OtherActor :type "Actor Object Reference") (OtherComp :type "PrimitiveComponent Object Reference") (OtherBodyIndex :type Integer))
  (cast `/Game/FirstPerson/Blueprints/BP_FirstPersonCharacter_Grab` OtherActor)
  (`SceneComponent.SetVisibility` (`self.text`) false false))

(fn `UserConstructionScript`)