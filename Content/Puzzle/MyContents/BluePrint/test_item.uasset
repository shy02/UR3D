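; Test item actor that can be removed from the puzzle game when the interaction flag is set while something is near it.
; A Sphere overlap shows or hides a Text component and sets or clears IsNear, with no filter on the overlapping actor.
; Tick destroys the actor once both IsPressed and IsNear are true.
; IsPressed is only reset on BeginPlay; nothing in this graph sets it true.
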(event `self.ReceiveBeginPlay`
  (set `self.isPressed` false)
  (set `self.isNear` false))

(event `self.ReceiveTick`
  (params (DeltaSeconds :type "Float (single-precision)"))
  (if (`self.isPressed`)
    (if (`self.isNear`)
      (`self.K2_DestroyActor`))))

(event `self.ReceiveActorBeginOverlap`
  (params (OtherActor :type "Actor Object Reference")))

(event `self.Sphere.OnComponentBeginOverlap`
  (params (OverlappedComponent :type "PrimitiveComponent Object Reference") (OtherActor :type "Actor Object Reference") (OtherComp :type "PrimitiveComponent Object Reference") (OtherBodyIndex :type Integer) (bFromSweep :type Boolean) (SweepResult :type "HitResult Structure (by ref)"))
  (`SceneComponent.SetVisibility` (`self.Text`) true false)
  (set `self.isNear` true))

(event `self.Sphere.OnComponentEndOverlap`
  (params (OverlappedComponent :type "PrimitiveComponent Object Reference") (OtherActor :type "Actor Object Reference") (OtherComp :type "PrimitiveComponent Object Reference") (OtherBodyIndex :type Integer))
  (`SceneComponent.SetVisibility` (`self.Text`) false false)
  (set `self.isNear` false))

(fn `UserConstructionScript`)