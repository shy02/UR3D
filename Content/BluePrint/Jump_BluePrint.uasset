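; A jump trigger actor that lifts the player when something overlaps it.
; On begin overlap it prints a debug string and instantly moves player pawn 0, with sweep, to a fixed height above its own location, whichever actor overlapped.
; An IsOver flag blocks repeat triggers until end overlap or BeginPlay clears it.
; IsJumpB is set and cleared alongside it but never read here.
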(event `self.ReceiveBeginPlay`
  (set `self.isOver` false :!label _label)
  (set `self.isJumpB` false))

(event `self.ReceiveActorEndOverlap`
  (params (OtherActor :type "Actor Object Reference"))
  (goto _label))

(event `self.ReceiveActorBeginOverlap`
  (params (OtherActor :type "Actor Object Reference"))
  (if (not (`self.isOver`))
    (`KismetSystemLibrary.PrintString` "Sliding")
    (bind _output_get (set `self.nextBlock` (+ (`self.K2_GetActorLocation`) (0.0 0.0 500.0))))
    (`self.K2_SetActorLocation` (`GameplayStatics.GetPlayerPawn` 0) _output_get true false) ; 지정된 위치로 이동
    (set `self.isOver` true)
    (set `self.isJumpB` true)))

(fn `UserConstructionScript`)