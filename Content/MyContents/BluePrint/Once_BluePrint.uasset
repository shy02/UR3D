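; A one-time crossing Blueprint that can be passed through once and then becomes a solid block.
; Block starts with collision off and the Stepped visual hidden, while begin overlap prints a debug string behind the IsOver and IsStepped flags.
; End overlap sets IsStepped, enables Block collision, disables Box collision and swaps the Cube visual for Stepped, with no path back.
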(event `self.ReceiveBeginPlay`
  (set `self.isOver` false)
  (`PrimitiveComponent.SetCollisionEnabled` (`self.Block`) "NoCollision")
  (`SceneComponent.SetVisibility` (`self.Stepped`) false false))

(event `self.ReceiveActorEndOverlap`
  (params (OtherActor :type "Actor Object Reference"))
  (set `self.isOver` false)
  (set `self.isStepped` true)
  (`PrimitiveComponent.SetCollisionEnabled` (`self.Block`) "QueryAndPhysics")
  (`PrimitiveComponent.SetCollisionEnabled` (`self.Box`) "NoCollision")
  (`SceneComponent.SetVisibility` (`self.Stepped`) true false)
  (`SceneComponent.SetVisibility` (`self.Cube`) false false))

(event `self.ReceiveActorBeginOverlap`
  (params (OtherActor :type "Actor Object Reference"))
  (if (`self.isStepped`)
    _
    (elif (not (`self.isOver`))
      (`KismetSystemLibrary.PrintString` "Once")
      (set `self.isOver` true))))

(fn `UserConstructionScript`)