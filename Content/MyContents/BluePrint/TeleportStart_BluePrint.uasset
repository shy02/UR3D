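; One-shot teleporter entrance actor that moves the player pawn to a TelePortEnd_BluePrint location.
; On BeginPlay it hides the Normal component and caches the location of a randomly picked end actor.
; The first overlap by any actor teleports player 0 there, then shows Normal and hides Cube.
; IsTeleport and IsOver, the latter set on end overlap, block any further teleports.
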(event `self.ReceiveBeginPlay`
  (set `self.isOver` false)
  (set `self.isTeleport` false)
  (`SceneComponent.SetVisibility` (`self.Normal`) false false)
  (bind _outactors (`GameplayStatics.GetAllActorsOfClass` "/Game/MyContents/BluePrint/TelePortEnd_BluePrint.TelePortEnd_BluePrint_C"))
  (set `self.teleportBlock` (`self.K2_GetActorLocation` (`KismetArrayLibrary.Array_Random` _outactors))))

(event `self.ReceiveActorEndOverlap`
  (params (OtherActor :type "Actor Object Reference"))
  (set `self.isOver` true))

(event `self.ReceiveActorBeginOverlap`
  (params (OtherActor :type "Actor Object Reference"))
  (if (`self.isOver`)
    _
    (elif (not (`self.isTeleport`))
      (`KismetSystemLibrary.PrintString` "Teleport")
      (`self.K2_SetActorLocation` (`GameplayStatics.GetPlayerPawn` 0) (`self.teleportBlock`) false true) ; 지정된 위치로 이동
      (set `self.isTeleport` true)
      (`SceneComponent.SetVisibility` (`self.Normal`) true false)
      (`SceneComponent.SetVisibility` (`self.Cube`) false false))))

(fn `UserConstructionScript`)