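; Start-point trigger actor that shows and starts an on-screen timer when overlaps occur.
; Beginning an overlap creates the Timer widget with its timer paused, unless the run is over or a timer exists; ending the overlap unpauses it and flags it as existing.
; StopTimer pauses that timer through GetParentValue, which exposes the widget and flag, alongside an IsParent flag set at BeginPlay.
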(event `self.ReceiveBeginPlay`
  (set `self.isOver` false)
  (set `self.isParent` true))

(event `self.ReceiveActorEndOverlap`
  (params (OtherActor :type "Actor Object Reference"))
  (`KismetSystemLibrary.K2_UnPauseTimer` (`self.timer_obj`) "Timer_")
  (set `self.isTimerExist` true))

(event `self.ReceiveActorBeginOverlap`
  (params (OtherActor :type "Actor Object Reference"))
  (if (`self.isOver`)
    _
    (elif (not (`self.isTimerExist`))
      (`KismetSystemLibrary.PrintString` "Timer Start")
      (`self.SetTimer`))))

(event `SetTimer`
  (bind _returnvalue (`|CreateWidget` "/Game/MyContents/BluePrint/Timer.Timer_C"))
  (bind _output_get (set `self.timer_obj` _returnvalue))
  (`UserWidget.AddToViewport` _output_get 0)
  (`KismetSystemLibrary.K2_PauseTimer` (`self.timer_obj`) "Timer_"))

(event `StopTimer`
  (`KismetSystemLibrary.PrintString` "Hello")
  (bind (_timerexist _obj) (`self.GetParentValue`))
  (`KismetSystemLibrary.K2_PauseTimer` _obj "Timer_"))

(fn `GetParentValue`
  (returns (TimerExist :type Boolean) (obj :type "/Game/MyContents/BluePrint/Timer Object Reference"))
  (return (`self.isTimerExist`) (`self.timer_obj`)))

(fn `UserConstructionScript`)