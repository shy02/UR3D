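; BP_FoodSpawnControl picks a random set of distinct food actors at BeginPlay and triggers FFOD on each.
; It gathers one actor from each of twelve BP_food child classes into Food, then draws INDEX times into BpFoodRequest.
; AddUnique's failure value, captured by re-adding the first element, detects duplicate draws, which retry until a new food is found.
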(event `self.ReceiveBeginPlay`
  (bind _bp_food_request (`self.bp_food_Request`))
  (bind _returnvalue (`GameplayStatics.GetActorOfClass` "/Game/12blue/BP_food_Child1.BP_food_Child1_C"))
  (bind _returnvalue_2 (`GameplayStatics.GetActorOfClass` "/Game/12blue/BP_food_Child2.BP_food_Child2_C"))
  (bind _returnvalue_3 (`GameplayStatics.GetActorOfClass` "/Game/12blue/BP_food_Child3.BP_food_Child3_C"))
  (bind _returnvalue_4 (`GameplayStatics.GetActorOfClass` "/Game/12blue/BP_food_Child4.BP_food_Child4_C"))
  (bind _returnvalue_5 (`GameplayStatics.GetActorOfClass` "/Game/12blue/BP_food_Child5.BP_food_Child5_C"))
  (bind _returnvalue_6 (`GameplayStatics.GetActorOfClass` "/Game/12blue/BP_food_Child6.BP_food_Child6_C"))
  (bind _returnvalue_7 (`GameplayStatics.GetActorOfClass` "/Game/12blue/BP_food_Child7.BP_food_Child7_C"))
  (bind _returnvalue_8 (`GameplayStatics.GetActorOfClass` "/Game/12blue/BP_food_Child8.BP_food_Child8_C"))
  (bind _returnvalue_9 (`GameplayStatics.GetActorOfClass` "/Game/12blue/BP_food_Child9.BP_food_Child9_C"))
  (bind _returnvalue_10 (`GameplayStatics.GetActorOfClass` "/Game/12blue/BP_food_Child91.BP_food_Child91_C"))
  (bind _returnvalue_11 (`GameplayStatics.GetActorOfClass` "/Game/12blue/BP_food_Child92.BP_food_Child92_C"))
  (bind _returnvalue_12 (`GameplayStatics.GetActorOfClass` "/Game/12blue/BP_food_Child93.BP_food_Child93_C"))
  (bind _output_get (set `self.food` (`|MakeArray` _returnvalue _returnvalue_2 _returnvalue_3 _returnvalue_4 _returnvalue_5 _returnvalue_6 _returnvalue_7 _returnvalue_8 _returnvalue_9 _returnvalue_10 _returnvalue_11 _returnvalue_12 :!type "/Game/12blue/BP_food Object Reference")))
  (bind _returnvalue_13 (`KismetArrayLibrary.Array_AddUnique` _output_get (`|GetArrayItem` _output_get)))
  (set `self.nope` _returnvalue_13)
  (for _ (range 1 (+ (`self.INDEX`) 1))
    (bind _returnvalue_14 (`KismetArrayLibrary.Array_AddUnique` (`self.bp_food_Request`) (`KismetArrayLibrary.Array_Random` (`self.food`)) :!label _label))
    (if (!= _returnvalue_14 (`self.nope`))
      (`/Game/12blue/BP_food.FFOD` (`|GetArrayItem` _bp_food_request (`KismetArrayLibrary.Array_LastIndex` _bp_food_request)))
      (else
        (goto _label)))))

(fn `UserConstructionScript`)