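; BP_food is a Mart actor with an overlap prompt and a blinking highlight light.
; Its widget, cone and point light start hidden, and the Box overlap shows or hides the widget.
; The FFOD event sets a flag that makes Tick reveal the light and flip its intensity on and off through a Delay scaled by frame time.
; Nothing here clears the flag or reveals the cone again.
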(event `self.ReceiveBeginPlay`
  (`SceneComponent.SetVisibility` (`self.Widget`) false false)
  (`SceneComponent.SetVisibility` (`self.Cone`) false false)
  (`SceneComponent.SetVisibility` (`self.PointLight`) false false))

(event `FFOD`
  (bind _output_get (set `self.bool` true)))

(event `self.ReceiveTick`
  (params (DeltaSeconds :type "Float (single-precision)"))
  (bind _pointlight (`self.PointLight`))
  (if (stale `FFOD` _output_get)
    (`SceneComponent.SetVisibility` (`self.PointLight`) true false)
    (`KismetSystemLibrary.Delay` (* DeltaSeconds 30.0))
    (`/Engine/EditorBlueprintResources/StandardMacros.FlipFlop`
      (:`A`
        (`LightComponent.SetIntensity` _pointlight (`self.0`)))
      (:`B`
        (`LightComponent.SetIntensity` _pointlight (`self.300`))))))

(event `self.Box.OnComponentBeginOverlap`
  (params (OverlappedComponent :type "PrimitiveComponent Object Reference") (OtherActor :type "Actor Object Reference") (OtherComp :type "PrimitiveComponent Object Reference") (OtherBodyIndex :type Integer) (bFromSweep :type Boolean) (SweepResult :type "HitResult Structure (by ref)"))
  (`SceneComponent.SetVisibility` (`self.Widget`) true false))

(event `self.Box.OnComponentEndOverlap`
  (params (OverlappedComponent :type "PrimitiveComponent Object Reference") (OtherActor :type "Actor Object Reference") (OtherComp :type "PrimitiveComponent Object Reference") (OtherBodyIndex :type Integer))
  (`SceneComponent.SetVisibility` (`self.Widget`) false false))

(fn `UserConstructionScript`)