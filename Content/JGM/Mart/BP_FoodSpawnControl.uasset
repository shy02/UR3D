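; BP_FoodSpawnControl picks a random set of unique food actors in the mart level and triggers each one.
; The construction script gathers the twelve BP_food_Child actors into an array and stores a duplicate AddUnique result as a failure sentinel.
; On BeginPlay it draws Index random foods, retrying on duplicates, and calls FFOD on each new pick.
; It then records each pick's position in the Food array into FoodIndex.
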(event `self.ReceiveBeginPlay`
  (bind _food_index (`self.food_index`))
  (bind _food_request (`self.food_Request`))
  ;[1 1 1] INDEX값 만큼 랜덤위치의 오브젝트 제어
  (for _ (range 1 (+ (`self.index`) 1))
    (bind _returnvalue (`KismetArrayLibrary.Array_AddUnique` (`self.food_Request`) (`KismetArrayLibrary.Array_Random` (`self.food`)) :!label _label))
    (if (!= _returnvalue (`self._Null`))
      (`/Game/JGM/Mart/BP_food.FFOD` (`|GetArrayItem` _food_request (`KismetArrayLibrary.Array_LastIndex` _food_request)))
      (else
        (goto _label))))
  (for _array_element (`self.food_Request`)
    (for (_array_element_2 _array_index) (`self.food`)
      (if (== _array_element _array_element_2)
        (`KismetArrayLibrary.Array_Set` _food_index (+ 1 (`KismetArrayLibrary.Array_LastIndex` _food_index)) _array_index true)
        (break)))))

(fn `UserConstructionScript`
  ;[1 1 1] 오브젝트를 모아 하나의 배열로 생성
  (bind _returnvalue (`GameplayStatics.GetActorOfClass` "/Game/JGM/Mart/BP_food_Child01.BP_food_Child01_C"))
  (bind _returnvalue_2 (`GameplayStatics.GetActorOfClass` "/Game/JGM/Mart/BP_food_Child02.BP_food_Child02_C"))
  (bind _returnvalue_3 (`GameplayStatics.GetActorOfClass` "/Game/JGM/Mart/BP_food_Child03.BP_food_Child03_C"))
  (bind _returnvalue_4 (`GameplayStatics.GetActorOfClass` "/Game/JGM/Mart/BP_food_Child04.BP_food_Child04_C"))
  (bind _returnvalue_5 (`GameplayStatics.GetActorOfClass` "/Game/JGM/Mart/BP_food_Child05.BP_food_Child05_C"))
  (bind _returnvalue_6 (`GameplayStatics.GetActorOfClass` "/Game/JGM/Mart/BP_food_Child06.BP_food_Child06_C"))
  (bind _returnvalue_7 (`GameplayStatics.GetActorOfClass` "/Game/JGM/Mart/BP_food_Child07.BP_food_Child07_C"))
  (bind _returnvalue_8 (`GameplayStatics.GetActorOfClass` "/Game/JGM/Mart/BP_food_Child08.BP_food_Child08_C"))
  (bind _returnvalue_9 (`GameplayStatics.GetActorOfClass` "/Game/JGM/Mart/BP_food_Child09.BP_food_Child09_C"))
  (bind _returnvalue_10 (`GameplayStatics.GetActorOfClass` "/Game/JGM/Mart/BP_food_Child10.BP_food_Child10_C"))
  (bind _returnvalue_11 (`GameplayStatics.GetActorOfClass` "/Game/JGM/Mart/BP_food_Child11.BP_food_Child11_C"))
  (bind _returnvalue_12 (`GameplayStatics.GetActorOfClass` "/Game/JGM/Mart/BP_food_Child12.BP_food_Child12_C"))
  (bind _output_get (set `self.food` (`|MakeArray` _returnvalue _returnvalue_2 _returnvalue_3 _returnvalue_4 _returnvalue_5 _returnvalue_6 _returnvalue_7 _returnvalue_8 _returnvalue_9 _returnvalue_10 _returnvalue_11 _returnvalue_12 :!type "/Game/JGM/Mart/BP_food Object Reference")))
  ;[1 1 1] Null값 생성
  (bind _returnvalue_13 (`KismetArrayLibrary.Array_AddUnique` _output_get (`|GetArrayItem` _output_get)))
  (set `self._Null` _returnvalue_13))