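; BP_toEnd is the checkout trigger in the mart level that decides whether the player's collected food matches the requested list.
; On overlap it refreshes the list counts from UI_MY (the cast game state), then compares the player's per-food counts against them using the spawn controller's FoodIndex.
; All matches, ANDed into a persistent flag, call Ending; otherwise it only prints "Reset".
; Its text label turns toward the player every tick.
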(event `self.ReceiveBeginPlay`
  (bind _asbp_first_person_character_shop (cast `/Game/JGM/BP_FirstPersonCharacter_SHOP` (`GameplayStatics.GetPlayerPawn` 0)))
  (set `self.Pawn` _asbp_first_person_character_shop)
  (bind _asui_my (cast `/Game/JGM/UI_MY` (`GameplayStatics.GetGameState`)))
  (set `self.ToUI` _asui_my)
  (bind _returnvalue (`GameplayStatics.GetActorOfClass` "/Game/JGM/Mart/BP_FoodSpawnControl.BP_FoodSpawnControl_C"))
  (set `self.FSC` _returnvalue))

(event `self.ReceiveTick`
  (params (DeltaSeconds :type "Float (single-precision)"))
  (`SceneComponent.K2_SetWorldRotation` (`self.TextRender`) (`KismetMathLibrary.FindLookAtRotation` (`SceneComponent.K2_GetComponentLocation` (`self.TextRender`)) (`self.K2_GetActorLocation` (`GameplayStatics.GetPlayerPawn` 0))) false false))

(event `self.ReceiveActorBeginOverlap`
  (params (OtherActor :type "Actor Object Reference"))
  (bind _andbool (`self.andbool`))
  ;[1 1 1] 목록 갯수 초기화
  (`/Game/JGM/UI_MY.copyRnd` (`self.ToUI`))
  (if (== OtherActor (`GameplayStatics.GetPlayerPawn` 0))
    (for (_array_element _array_index) (`/Game/JGM/Mart/BP_FoodSpawnControl.food_index` (`self.FSC`))
      (`KismetArrayLibrary.Array_Set` (`self.NewVar`) _array_index (== (`|GetArrayItem` (`/Game/JGM/BP_FirstPersonCharacter_SHOP.FoodTriggerCount` (`self.Pawn`)) _array_element) (`|GetArrayItem` (`/Game/JGM/UI_MY.setRnd` (`self.ToUI`)) _array_index)) true))
    (for _array_element_2 (`self.NewVar`)
      (set `self.andbool` (and _array_element_2 _andbool)))
    (if _andbool
      (`/Game/JGM/UI_MY.ending` (`self.ToUI`))
      (else
        (`KismetSystemLibrary.PrintString` "Reset")))))

(fn `UserConstructionScript`)