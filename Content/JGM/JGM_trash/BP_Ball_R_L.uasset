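; BP_Ball_R_L is an actor that shifts its Sphere component according to where the player pawn is relative to its Cube component.
; Each tick it sets the Sphere's relative location to the Cube-to-player vector scaled by NewVar, so the offset grows with player distance.
; It also prints that vector and the player location every tick as debug output.
; A disconnected world-location variant measured from the Sphere itself remains in the graph.
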(event `self.ReceiveTick`
  (params (DeltaSeconds :type "Float (single-precision)"))
  (bind _returnvalue (`self.K2_GetActorLocation` (`GameplayStatics.GetPlayerPawn` 0)))
  (bind _returnvalue_2 (- _returnvalue (`SceneComponent.K2_GetComponentLocation` (`self.Cube`))))
  (`SceneComponent.K2_SetRelativeLocation` (`self.Sphere`) (* _returnvalue_2 (`self.NewVar`)) false false)
  (`KismetSystemLibrary.PrintString` (`KismetStringLibrary.Conv_VectorToString` _returnvalue_2) true true (struct :`G` 0.66 :`B` 1.0 :`A` 1.0) 2.0 "1")
  (`KismetSystemLibrary.PrintString` (`KismetStringLibrary.Conv_VectorToString` _returnvalue) true true (struct :`G` 0.66 :`B` 1.0 :`A` 1.0) 2.0 "2"))

(fn `UserConstructionScript`)