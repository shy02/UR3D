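; BP_SpawnControl is an actor that, on overlap, triggers spawning at randomly chosen BP_TargeT actors gathered at BeginPlay.
; It loops over a Things range, adding random targets to a list with AddUnique, then calls SpawnThing on every listed target.
; Duplicates are detected against a cached failed-AddUnique result and retried until a shared counter reaches the target count.
; The picked list is never cleared between overlaps.
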(event `spawn_dump`
  (for _ (range (`self.Things_init`) (+ (`self.Things`) 1)) :!label _label
    (bind _returnvalue (`KismetArrayLibrary.Array_AddUnique` (`self.BP_DUMP_target`) (`KismetArrayLibrary.Array_Random` (`self.BP_target`)) :!label _label_2))
    (bind _output_get (set `self.Things_bool` (!= _returnvalue (`self.NO`))))
    (if (not _output_get)
      (bind _output_get_2 (set `self.Routine` (+ (`self.Routine`) 1)))
      (if (== _output_get_2 (`KismetArrayLibrary.Array_Length` (`self.BP_target`)))
        (`KismetSystemLibrary.PrintString` "IS FUll")
        (set `self.Routine` 1)
        (else
          (goto _label_2)))))
  (for _array_element (`self.BP_DUMP_target`)
    (`/Game/JGM/JGM_trash/BP_TargeT.spawnThing` _array_element))
  (`KismetSystemLibrary.PrintString` "Spawn complete"))

(event `self.ReceiveActorBeginOverlap`
  (params (OtherActor :type "Actor Object Reference"))
  (goto _label))

(event `self.ReceiveBeginPlay`
  (bind _bp_target (`self.BP_target`))
  ;[1 1 1] 시작시 초기화 하는것들
  (bind _outactors (`GameplayStatics.GetAllActorsOfClass` "/Game/JGM/JGM_trash/BP_TargeT.BP_TargeT_C"))
  (bind _output_get (set `self.BP_target` _outactors))
  (`KismetSystemLibrary.PrintString` (`KismetStringLibrary.Conv_IntToString` (`KismetArrayLibrary.Array_Length` _output_get)))
  ;[1 1 1] null값으로 초기화
  (bind _returnvalue (`KismetArrayLibrary.Array_AddUnique` _bp_target (`|GetArrayItem` _bp_target)))
  (set `self.NO` _returnvalue))

(fn `UserConstructionScript`)