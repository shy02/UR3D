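; BP_trash_M is a trash actor in the TrashMan content that can be removed while something overlaps its box.
; Box overlap begin and end toggle a prompt widget, hidden at BeginPlay, and the IsOverlap flag.
; DestroyTrash checks that flag, calls DestroyParent on the BP_trashTargetArray actor found in the level, then destroys itself.
; Disconnected leftover logic would make a TextRender face and follow the player.
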(event `self.ReceiveBeginPlay`
  (`SceneComponent.SetVisibility` (`self.Widget`) false false))

(event `self.ReceiveTick`
  (params (DeltaSeconds :type "Float (single-precision)")))

(event `DestroyTrash`
  (if (`self.isOverlap`)
    (bind _returnvalue (`GameplayStatics.GetActorOfClass` "/Game/JGM/TrashMan/BP_trashTargetArray.BP_trashTargetArray_C"))
    (`/Game/JGM/TrashMan/BP_trashTargetArray.DestroyParent` _returnvalue)
    (`self.K2_DestroyActor`)))

(event `self.Box.OnComponentBeginOverlap`
  (params (OverlappedComponent :type "PrimitiveComponent Object Reference") (OtherActor :type "Actor Object Reference") (OtherComp :type "PrimitiveComponent Object Reference") (OtherBodyIndex :type Integer) (bFromSweep :type Boolean) (SweepResult :type "HitResult Structure (by ref)"))
  (`SceneComponent.SetVisibility` (`self.Widget`) true false)
  (set `self.isOverlap` true))

(event `self.Box.OnComponentEndOverlap`
  (params (OverlappedComponent :type "PrimitiveComponent Object Reference") (OtherActor :type "Actor Object Reference") (OtherComp :type "PrimitiveComponent Object Reference") (OtherBodyIndex :type Integer))
  (`SceneComponent.SetVisibility` (`self.Widget`) false false)
  (set `self.isOverlap` false))

(fn `UserConstructionScript`)