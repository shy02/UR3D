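; BP_trashTargetArray scatters three trash types at random across every BP_trashTarget placed in the level.
; Its construction script gathers and attaches those targets to itself and sets a per-type limit from a third of their count.
; On BeginPlay it rolls a type for each target and spawns that trash at the target's transform, re-rolling when that type's counter exceeds the limit, keeping the mix roughly even.
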(event `self.ReceiveBeginPlay`
  (for (_ _array_index) (`self.Out Actors`)
    (bind _output_get (set `self.rndInteger` (`KismetMathLibrary.RandomIntegerInRange` 0 2) :!label _label))
    (`KismetSystemLibrary.PrintString` (`KismetStringLibrary.Conv_IntToString` _output_get))
    (if (and (>= (`self.arrayLengthDivid`) (`self.item01`)) (== (`self.rndInteger`) 0))
      (bind _returnvalue (`self.GetTransform` (`|GetArrayItem` (`self.Out Actors`) _array_index)))
      (`|SpawnActorFromClass` "/Game/JGM/TrashMan/BP_trash_01.BP_trash_01_C" _returnvalue "Undefined" "OverrideRootScale" null null)
      (set `self.item01` (+ (`self.item01`) 1))
      (elif (and (>= (`self.arrayLengthDivid`) (`self.item02`)) (== (`self.rndInteger`) 1))
        (`|SpawnActorFromClass` "/Game/JGM/TrashMan/BP_trash_02.BP_trash_02_C" _returnvalue "Undefined" "OverrideRootScale" null null)
        (set `self.item02` (+ (`self.item02`) 1))
        (elif (and (>= (`self.arrayLengthDivid`) (`self.item03`)) (== (`self.rndInteger`) 2))
          (`|SpawnActorFromClass` "/Game/JGM/TrashMan/BP_trash_03.BP_trash_03_C" _returnvalue "Undefined" "OverrideRootScale" null null)
          (set `self.item03` (+ (`self.item03`) 1))
          (else
            (`KismetSystemLibrary.PrintString` "Failed")
            (goto _label)))))))

(fn `UserConstructionScript`
  (`KismetArrayLibrary.Array_Clear` (`self.Out Actors`))
  (bind _outactors (`GameplayStatics.GetAllActorsOfClass` "/Game/JGM/TrashMan/BP_trashTarget.BP_trashTarget_C"))
  (bind _output_get (set `self.Out Actors` _outactors))
  (for _array_element _output_get
    (`self.K2_AttachToActor` _array_element self "None" "KeepWorld" "KeepWorld" "KeepWorld" true)
    (set `self.arrayLengthDivid` (/ (`KismetArrayLibrary.Array_Length` (`self.Out Actors`)) 3))))