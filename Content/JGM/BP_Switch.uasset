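; BP_Switch is a two-way teleport actor that moves the player between its Start and End components.
; Overlap events on both components set flags, and the Trick event uses them to send the player pawn to the opposite component's location.
; Each jump calls TrickNum on the first-person shop character; if that character's Trigg count is zero or less, Trick calls Ending on UI_MY, cast from the GameState, instead.
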(event `self.ReceiveBeginPlay`
  ;[1 1 1] 변수들 초기화
  (bind _asui_my (cast `/Game/JGM/UI_MY` (`GameplayStatics.GetGameState`)))
  (set `self.UI` _asui_my)
  (bind _asbp_first_person_character_shop (cast `/Game/JGM/BP_FirstPersonCharacter_SHOP` (`GameplayStatics.GetPlayerPawn` 0)))
  (set `self.FIrst` _asbp_first_person_character_shop))

(event `Trick`
  (bind _returnvalue (`GameplayStatics.GetPlayerPawn` 0))
  ;[1 1 1] 서로 교환
  (if (<= (`/Game/JGM/BP_FirstPersonCharacter_SHOP.Trigg` (`self.FIrst`)) 0)
    (`/Game/JGM/UI_MY.ending` (`self.UI`))
    (elif (`self.start_B`)
      (`self.K2_SetActorLocation` _returnvalue (`SceneComponent.K2_GetComponentLocation` (`self.End`)) false false)
      (`/Game/JGM/BP_FirstPersonCharacter_SHOP.TrickNum` (`self.FIrst`) :!label _label)
      (elif (`self.end_B`)
        (`self.K2_SetActorLocation` _returnvalue (`SceneComponent.K2_GetComponentLocation` (`self.Start`)) false false)
        (goto _label)))))

(event `self.Start.OnComponentBeginOverlap`
  (params (OverlappedComponent :type "PrimitiveComponent Object Reference") (OtherActor :type "Actor Object Reference") (OtherComp :type "PrimitiveComponent Object Reference") (OtherBodyIndex :type Integer) (bFromSweep :type Boolean) (SweepResult :type "HitResult Structure (by ref)"))
  ;[1 1 1] actor와 충돌시 상호작용 가능한 bool 값처리
  (set `self.start_B` true)
  (`KismetSystemLibrary.PrintString` "Start"))

(event `self.End.OnComponentBeginOverlap`
  (params (OverlappedComponent :type "PrimitiveComponent Object Reference") (OtherActor :type "Actor Object Reference") (OtherComp :type "PrimitiveComponent Object Reference") (OtherBodyIndex :type Integer) (bFromSweep :type Boolean) (SweepResult :type "HitResult Structure (by ref)"))
  ;[1 1 1] actor와 충돌시 상호작용 가능한 bool 값처리
  (set `self.end_B` true)
  (`KismetSystemLibrary.PrintString` "End"))

(event `self.End.OnComponentEndOverlap`
  (params (OverlappedComponent :type "PrimitiveComponent Object Reference") (OtherActor :type "Actor Object Reference") (OtherComp :type "PrimitiveComponent Object Reference") (OtherBodyIndex :type Integer))
  ;[1 1 1] actor와 충돌시 상호작용 가능한 bool 값처리
  (set `self.end_B` false)
  (`KismetSystemLibrary.PrintString` "End2"))

(event `self.Start.OnComponentEndOverlap`
  (params (OverlappedComponent :type "PrimitiveComponent Object Reference") (OtherActor :type "Actor Object Reference") (OtherComp :type "PrimitiveComponent Object Reference") (OtherBodyIndex :type Integer))
  ;[1 1 1] actor와 충돌시 상호작용 가능한 bool 값처리
  (set `self.start_B` false)
  (`KismetSystemLibrary.PrintString` "Start2"))

(fn `UserConstructionScript`)